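; BP_GM_MainChar, apparently the main character's game mode, handles saving the player's position and restarting the level.
; SaveGame writes the BP_MainChar transform into the existing BP_SaveGame in slot "save1".
; LoadGame and RestartLevel restart through console commands; RestartLevel first sends "save1" as a command, deleting nothing itself.
; Logic to restore the transform or create a missing save is disconnected, and BeginPlay is empty, so nothing here applies saves.
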(event Custom|SaveGame
  ;[1 1 1] 게임 저장
  (bind _returnvalue (SaveGame|LoadGamefromSlot "save1"))
  (bind _asbp_save_game (Utilities|Casting|CastToBP_SaveGame _returnvalue))
  (Variables|/Game/System/BP_SaveGame.BP_SaveGame_C|SetSaveGame_LoadGame _asbp_save_game (Transformation|GetActorTransform (.AsBP%20Main%20Char (Utilities|Casting|CastToBP_MainChar (Game|GetPlayerCharacter 0)))))
  (SaveGame|SaveGametoSlot _asbp_save_game "save1"))

(event Custom|LoadGame
  ;[1 1 1] 기존 게임 불러오기
  (Development|ExecuteConsoleCommand "RestartLevel" 0))

(event Custom|RestartLevel
  ;[1 1 1] 세이브 파일 삭제 후 재생성
  (Development|ExecuteConsoleCommand "save1" 0)
  (Development|ExecuteConsoleCommand "RestartLevel" 0))

(event EventBeginPlay)

(fn ConstructionScript)