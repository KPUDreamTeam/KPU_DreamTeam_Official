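; Boss character Blueprint that repeats a scripted spell attack from BeginPlay.
; Attack plays the first spell montage section, spawns a magic circle and runs the Javellings macro, which spawns three laterally offset attack actors with staggered charge values.
; After delays it plays the second montage section, then calls Attack again.
; SwordSlam and Stone define alternative attack spawns but are never executed.
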(event Custom|Attack
  (Animation|Montage|PlayMontage (Variables|Character|GetMesh) "/Game/Character/Character/Boss/Animation/Animation/Montage/AM_Char_Boss_Spell.AM_Char_Boss_Spell" 1.0 0.0 "Spell_0"
    (:then
      (Game|SpawnActorfromClass "/Game/Character/Character/Boss/BP_Boss_MagicCircle.BP_Boss_MagicCircle_C" (Math|Transform|MakeTransform (+ (Transformation|GetActorLocation) (Variables|Default|GetMagicAttackLocation)) "0, 0, 0" "1,1,1") "Undefined" 0 0)
      (|Javellings
        (:OutputPin
          (Utilities|FlowControl|Delay 3.3)
          (Animation|Montage|PlayMontage (Variables|Character|GetMesh) "/Game/Character/Character/Boss/Animation/Animation/Montage/AM_Char_Boss_Spell.AM_Char_Boss_Spell" 1.0 0.0 "Spell_1"
            (:then
              (Utilities|FlowControl|Delay 1e+01)
              (CallFunction|Attack))))))))

(event EventBeginPlay
  (CallFunction|Attack))

(fn ConstructionScript)