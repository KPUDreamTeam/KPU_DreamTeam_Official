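; Boss sword attack actor that, when charged, slashes toward the player and then removes itself.
; It yaws toward the player every tick while the sword fades in through a material mask and winds up, then stops tracking and pitches down with a camera shake.
; Sword overlaps send a boss-hit interface message only during that swing.
; A threshold timeline then fades the sword out before a short lifespan destroys the actor.
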(event OnComponentBeginOverlap(SwordCollision)
  (params (OverlappedComponent :type Primitive%20Component%20Object%20Reference) (OtherActor :type Actor%20Object%20Reference) (OtherComp :type Primitive%20Component%20Object%20Reference) (OtherBodyIndex :type Integer) (bFromSweep :type Boolean) (SweepResult :type Hit%20Result%20Structure%20%28by%20ref%29))
  (if (Variables|Default|GetbIsAttacking?)
    (Class|BPIBoss|BPIBossHit(Message) OtherActor (Transformation|GetActorLocation))))

(event Custom|FadeIn
  (bind _mask (Timeline|Timeline_FadeIn PlayFromStart)
    (:Update
      (Rendering|Material|SetScalarParameterValueonMaterials (Variables|Default|GetSword) "Mask" _mask))
    (:Finished
      (CallFunction|LaunchAttack))))

(event Custom|LaunchAttack
  (bind _sword (Variables|Default|GetSword))
  (bind _rootcomponent (Variables|Transformation|GetRootComponent))
  (bind _rootcomponent_2 (Variables|Transformation|GetRootComponent))
  (bind _relativelocation (Variables|/Script/Engine.SceneComponent|GetRelativeLocation _rootcomponent))
  (bind _relativerotation (Variables|/Script/Engine.SceneComponent|GetRelativeRotation _rootcomponent_2))
  (bind _relativerotation_2 (Variables|/Script/Engine.SceneComponent|GetRelativeRotation _sword))
  (Components|MoveComponentTo _sword (Variables|/Script/Engine.SceneComponent|GetRelativeLocation _sword) (Math|Rotator|MakeRotator (.roll _relativerotation_2) (.pitch _relativerotation_2) (- (.yaw _relativerotation_2) 9e+01)) true true 0.4 false)
  (Utilities|FlowControl|Delay 0.5)
  (Audio|PlaySoundatLocation "/Game/Character/Character/Boss/Sound/SFX_Boss_Sword_1.SFX_Boss_Sword_1" _relativelocation "0, 0, 0" 1.0 1.0 0.0 0 0 0)
  (Utilities|FlowControl|Delay 0.5)
  (Actor|Tick|SetActorTickEnabled false)
  (Camera|PlayWorldCameraShake "/Game/Character/Character/Boss/BP_CameraShake_Boss.BP_CameraShake_Boss_C" _relativelocation 5e+02 5e+03)
  (Variables|Default|SetbIsAttacking? true)
  (Components|MoveComponentTo _rootcomponent_2 (Variables|/Script/Engine.SceneComponent|GetRelativeLocation _rootcomponent_2) (Math|Rotator|MakeRotator (.roll _relativerotation) (- (.pitch _relativerotation) 9e+01) (.yaw _relativerotation)) true true 0.3 false)
  (Variables|Default|SetbIsAttacking? false)
  (Utilities|FlowControl|Delay 2.0)
  (CallFunction|FadeOut))

(event Custom|FadeOut
  (bind _fadeoutamount (Timeline|Timeline_FadeOut Play)
    (:Update
      (Rendering|Material|SetScalarParameterValueonMaterials (Variables|Default|GetSword) "Alpha Threshold (S)" _fadeoutamount))
    (:Finished
      (Utilities|FlowControl|Delay 0.2)
      (Actor|SetLifeSpan 1.0))))

(event Custom|Charge
  (CallFunction|Fadein))

(event EventBeginPlay)

(event EventTick
  (params (DeltaSeconds :type Float%20%28single-precision%29))
  (Transformation|SetActorRotation (Math|Rotator|MakeRotator 0.0 0.0 (.yaw (Math|Rotator|FindLookatRotation (Transformation|GetActorLocation) (Transformation|GetActorLocation (Game|GetPlayerCharacter 0)))))))

(fn ConstructionScript)