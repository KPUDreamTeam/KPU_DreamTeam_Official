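; Boss attack actor with a sword that tracks the player, then hurls itself at their position.
; BeginPlay calls Charge, and Tick keeps it facing the player until LaunchAttack disables ticking.
; SetTarget line-traces toward the player's offset position, stopping at blocking geometry, and shows a fading decal as a one-second warning.
; The actor then lunges there with sound and camera shake, flagged as attacking during the move, before fading out.
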(event EventBeginPlay
  (|CallParentFunction)
  (CallFunction|Charge 0.0))

(event Collision|EventActorBeginOverlap
  (params (OtherActor :type Actor%20Object%20Reference)))

(event EventTick
  (params (DeltaSeconds :type Float%20%28single-precision%29))
  (Transformation|SetActorRotation (Math|Rotator|FindLookatRotation (Transformation|GetActorLocation) (Transformation|GetActorLocation (Game|GetPlayerCharacter 0)))))

(event EventLaunchAttack
  (bind _sword (Variables|Default|GetSword))
  (bind _rootcomponent (Variables|Transformation|GetRootComponent))
  (bind _relativelocation (Variables|/Script/Engine.SceneComponent|GetRelativeLocation _rootcomponent))
  (Components|MoveComponentTo _sword (Variables|/Script/Engine.SceneComponent|GetRelativeLocation _sword) (Variables|/Script/Engine.SceneComponent|GetRelativeRotation _sword) true true 0.4 false)
  (Utilities|FlowControl|Delay 0.5)
  (|SetTarget)
  (Audio|PlaySoundatLocation "/Game/Character/Character/Boss/Sound/SFX_Boss_Rock_0.SFX_Boss_Rock_0" _relativelocation "0, 0, 0" 1.0 1.0 0.0 0 0 0)
  (Actor|Tick|SetActorTickEnabled false)
  (Camera|PlayWorldCameraShake "/Game/Character/Character/Boss/BP_CameraShake_Boss.BP_CameraShake_Boss_C" _relativelocation 5e+02 5e+03)
  (Variables|Default|SetbIsAttacking? true)
  (Components|MoveComponentTo (Variables|Transformation|GetRootComponent) (Variables|Default|GetTarget) (Math|Rotator|FindLookatRotation (Transformation|GetActorLocation) (Variables|Default|GetTarget)) true true 0.3 false)
  (Variables|Default|SetbIsAttacking? false)
  (Utilities|FlowControl|Delay 2.0)
  (CallFunction|FadeOut))

(fn ConstructionScript
  (|CallParentFunction))