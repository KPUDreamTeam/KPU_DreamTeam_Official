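; BP_Boss_MagicCircle is a short-lived magic circle effect actor for the boss.
; On BeginPlay it fades in, waits, fades out, then destroys itself a couple of seconds later.
; Two timelines drive the Opacity scalar parameter on the MagicCircle component's materials.
; Every Tick it sets its yaw to face the player character.
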(event Custom|FadeOut
  (bind _newtrack_0 (Timeline|FadeOutTimeline Play)
    (:Update
      (Rendering|Material|SetScalarParameterValueonMaterials (Variables|Default|GetMagicCircle) "Opacity" _newtrack_0))))

(event Custom|FadeIn
  (bind _newtrack_0 (Timeline|FadeInTimeline Play)
    (:Update
      (Rendering|Material|SetScalarParameterValueonMaterials (Variables|Default|GetMagicCircle) "Opacity" _newtrack_0))))

(event EventBeginPlay
  (CallFunction|Fadein)
  (Utilities|FlowControl|Delay 2.0)
  (CallFunction|FadeOut)
  (Utilities|FlowControl|Delay 2.0)
  (Actor|DestroyActor))

(event EventTick
  (params (DeltaSeconds :type Float%20%28single-precision%29))
  (Transformation|SetActorRotation (Math|Rotator|MakeRotator 0.0 0.0 (.yaw (Math|Rotator|FindLookatRotation (Transformation|GetActorLocation) (Transformation|GetActorLocation (Game|GetPlayerCharacter 0)))))))

(fn ConstructionScript)