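; Default zombie character that tracks player detection, sight and attack range through boolean flags and a detection widget.
; The widget starts hidden, and custom events set the detected and in-sight flags.
; Capsule overlap with BP_MainChar clears detection, hides the widget and enables the zombie's attack flag.
; Ending that overlap sets IsZombieCanAttackChar to true on the player instead of clearing the zombie's own flag.
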(event OnComponentBeginOverlap(CapsuleComponent)
  (params (OverlappedComponent :type Primitive%20Component%20Object%20Reference) (OtherActor :type Actor%20Object%20Reference) (OtherComp :type Primitive%20Component%20Object%20Reference) (OtherBodyIndex :type Integer) (bFromSweep :type Boolean) (SweepResult :type Hit%20Result%20Structure%20%28by%20ref%29))
  (Utilities|Casting|CastToBP_MainChar OtherActor)
  (Variables|Default|SetbIsZombieDetectChar? false)
  (CallFunction|WidgetVisibility)
  (Variables|Default|SetbIsZombieCanAttackChar? true))

(event OnComponentEndOverlap(CapsuleComponent)
  (params (OverlappedComponent :type Primitive%20Component%20Object%20Reference) (OtherActor :type Actor%20Object%20Reference) (OtherComp :type Primitive%20Component%20Object%20Reference) (OtherBodyIndex :type Integer))
  (bind _asbp_main_char (Utilities|Casting|CastToBP_MainChar OtherActor))
  (Variables|/Game/Character/MainCharacter/BP_MainChar.BP_MainChar_C|SetbIsZombieCanAttackChar? _asbp_main_char true))

(event Custom|WidgetVisibility
  (Rendering|SetVisibility (Variables|Default|GetDetectWidget) false false))

(event EventBeginPlay
  (Rendering|SetVisibility (Variables|Default|GetDetectWidget) false false))

(event EventCharinSight
  (Variables|Default|SetbIsCharInSight? true))

(event EventDetectChar
  (Variables|Default|SetbIsZombieDetectChar? true))

(fn ConstructionScript)