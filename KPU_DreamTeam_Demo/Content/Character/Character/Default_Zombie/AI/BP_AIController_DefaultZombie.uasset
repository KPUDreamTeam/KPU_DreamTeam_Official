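; AI controller for the default zombie that runs its behavior tree on possession and tracks perceived characters.
; AI perception updates filter for actors tagged "Character" and store a sensed one as the MainCharacter blackboard target.
; When perception is lost, it clears the target, saves the actor's current location as LastLocation and sets bGoToLocation for the tree to use.
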(event OnTargetPerceptionUpdated(AIPerception)
  (params (Actor :type Actor%20Object%20Reference) (Stimulus :type AI%20Stimulus%20Structure))
  (bind _output_get (Variables|Default|SetPerceptionActor Actor))
  (if (Actor|ActorHasTag _output_get "Character")
    (if (.bSuccessfullySensed (Utilities|Struct|BreakAIStimulus Stimulus))
      (AI|Components|Blackboard|SetValueasObject (Variables|Default|GetBlackboard) (Utilities|Name|MakeLiteralName "MainCharacter") (Variables|Default|GetPerceptionActor))
      (else
        (bind _output_get_2 (Variables|Default|SetActorLastLocation (Transformation|GetActorLocation (Variables|Default|GetPerceptionActor))))
        (AI|Components|Blackboard|SetValueasBool (Variables|Default|GetBlackboard) (Utilities|Name|MakeLiteralName "bGoToLocation") true)
        (AI|Components|Blackboard|SetValueasVector (Variables|Default|GetBlackboard) (Utilities|Name|MakeLiteralName "LastLocation") _output_get_2)
        (AI|Components|Blackboard|SetValueasObject (Variables|Default|GetBlackboard) (Utilities|Name|MakeLiteralName "MainCharacter") 0)))))

(event EventBeginPlay)

(event EventTick
  (params (DeltaSeconds :type Float%20%28single-precision%29)))

(event EventPossess
  (params (PossessedPawn :type Pawn%20Object%20Reference))
  (AI|RunBehaviorTree "/Game/Character/Character/Default_Zombie/AI/BT_DefaultZombie.BT_DefaultZombie")
  (AI|Components|Blackboard|SetValueasBool (Variables|Default|GetBlackboard) (Utilities|Name|MakeLiteralName "bGoToLocation") false))

(fn ConstructionScript)