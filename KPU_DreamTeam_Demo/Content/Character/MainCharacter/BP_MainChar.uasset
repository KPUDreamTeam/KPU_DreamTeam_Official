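; Player character Blueprint with walking, sprint, free look, swimming, wall climbing and weapon equip, plus a stats widget.
; Jump alternates between jump-and-climb and release; climbing snaps the capsule to traced wall hits in Flying mode, where MoveOnWall steers along the surface.
; Tick compares depth below the recorded water-entry Z with capsule size to switch Swimming/Walking, toggling the physics volume's water flag.
; Interaction inside an equip area reveals the weapon.
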(event EventBeginPlay
  (Utilities|FlowControl|Sequence
    (:then_0
      (bind _returnvalue (UserInterface|CreateWidget "/Game/HUD/UI_Character_Stats.UI_Character_Stats_C"))
      (UserInterface|Viewport|AddtoViewport _returnvalue 0))
    (:then_1
      (Rendering|SetVisibility (Variables|Default|GetCharacterWeapon) false false)
      (Variables|Default|SetbIsEnableCombatCollision? false))))

(event EventTick
  (params (DeltaSeconds :type Float%20%28single-precision%29))
  (|CheckSwimming))

(event EventEnterWater
  (Variables|Default|SetbIsInWater? true)
  (Variables|Default|SetMainCharWaterZ (.z (Transformation|GetActorLocation))))

(event EventExitWater
  (Variables|Default|SetbIsInWater? false))

(event EventCallFuncClimbing
  (bind _linetraceheadhit (Utilities|LineTracetoDetactWall (Variables|Default|GetLineTraceInputOffset)))
  (Utilities|FlowControl|Delay 0.2)
  (Pawn|Components|CharacterMovement|SetMovementMode (Variables|Character|GetCharacterMovement) "MOVE_Flying" 0)
  (Class|BPICharacterMovement|SetonWall(Message) (Components|SkeletalMesh|GetAnimInstance (Variables|Character|GetMesh)) true)
  (Components|Movement|StopMovementImmediately (Variables|Character|GetCharacterMovement))
  (Variables|/Script/Engine.CharacterMovementComponent|SetbOrientRotationToMovement (Variables|Character|GetCharacterMovement) false)
  (Components|MoveComponentTo (Variables|Collision|GetCapsuleComponent) (+ (.Location (Collision|BreakHitResult _linetraceheadhit)) (* (.Normal (Collision|BreakHitResult _linetraceheadhit)) (Variables|Default|GetClimbingWallDistance))) (Math|Rotator|MakeRotator 0.0 0.0 (.yaw (Math|Conversions|RotationFromXVector (* (.Normal (Collision|BreakHitResult _linetraceheadhit)) -1.0)))) false false 0.2 false))

(event Input|ActionEvents|InputActionSprint
  (params (Key :type Key%20Structure :default "None"))
  (bind _charactermovement (Variables|Character|GetCharacterMovement))
  ;[1 1 1] LeftShift를 통한 캐릭터 뛰기
  (:Pressed
    (Variables|/Script/Engine.CharacterMovementComponent|SetMaxWalkSpeed _charactermovement 4.5e+02)
    (Variables|Default|SetbIsSprinting? true))
  (:Released
    (Variables|/Script/Engine.CharacterMovementComponent|SetMaxWalkSpeed _charactermovement 3e+02)
    (Variables|Default|SetbIsSprinting? false)))

(event Input|ActionEvents|InputActionJump
  (params (Key :type Key%20Structure :default "None"))
  ;[1 1 1] 점프&벽타기
  (:Pressed
    (Utilities|FlowControl|FlipFlop
      (:A
        (switch Utilities|FlowControl|Switch|SwitchonEMovementMode (Variables|/Script/Engine.CharacterMovementComponent|GetMovementMode (Variables|Character|GetCharacterMovement))
          (:MOVE_Walking
            (Character|Jump)
            (CallFunction|CallFuncClimbing))))
      (:B
        (Pawn|Components|CharacterMovement|SetMovementMode (Variables|Character|GetCharacterMovement) "MOVE_Falling" 0)
        (Variables|/Script/Engine.CharacterMovementComponent|SetbOrientRotationToMovement (Variables|Character|GetCharacterMovement) true)
        (Class|BPICharacterMovement|SetonWall(Message) (Components|SkeletalMesh|GetAnimInstance (Variables|Character|GetMesh)) false))))
  (:Released
    (Character|StopJumping)))

(event Input|ActionEvents|InputActionFreeLook
  (params (Key :type Key%20Structure :default "None"))
  ;[1 1 1] Alt키를 통한 자유이동
  (:Pressed
    (Variables|Default|SetbFreeLook? true))
  (:Released
    (Variables|Default|SetbFreeLook? false)))

(event Input|AxisEvents|InputAxisMoveForward
  (params (AxisValue :type Float%20%28single-precision%29))
  ;[1 1 1] 이동키를 통한 벽타기
  (Variables|Default|SetMoveForwardAxisValue AxisValue)
  (switch Utilities|FlowControl|Switch|SwitchonEMovementMode (Variables|/Script/Engine.CharacterMovementComponent|GetMovementMode (Variables|Character|GetCharacterMovement))
    (:MOVE_Walking
      (if (Variables|Default|GetbFreeLook?) :!label _label
        ;[1 1 1] Alt키를 통한 자유이동
        (Pawn|Input|AddMovementInput (Math|Vector|GetForwardVector (Math|Rotator|MakeRotator 0.0 0.0 (.Yaw (Math|Rotator|BreakRotator (Transformation|GetWorldRotation (Variables|Collision|GetCapsuleComponent)))))) (Variables|Default|GetMoveForwardAxisValue) false)
        (else
          ;[1 1 1] 기본 이동
          (Pawn|Input|AddMovementInput (Math|Vector|GetForwardVector (Math|Rotator|MakeRotator 0.0 0.0 (.Yaw (Math|Rotator|BreakRotator (Pawn|GetControlRotation :!class /Script/Engine.Pawn))))) (Variables|Default|GetMoveForwardAxisValue) false))))
    (:MOVE_Swimming
      (goto _label))
    (:MOVE_Flying
      (CallFunction|MoveonWall (Transformation|GetActorUpVector) (Variables|Default|GetMoveForwardAxisValue)))))

(event Input|AxisEvents|InputAxisMoveRight
  (params (AxisValue :type Float%20%28single-precision%29))
  ;[1 1 1] 이동키를 통한 벽타기
  (Variables|Default|SetMoveRightAxisValue AxisValue)
  (switch Utilities|FlowControl|Switch|SwitchonEMovementMode (Variables|/Script/Engine.CharacterMovementComponent|GetMovementMode (Variables|Character|GetCharacterMovement))
    (:MOVE_Walking
      (if (Variables|Default|GetbFreeLook?) :!label _label
        ;[1 1 1] Alt키를 통한 자유이동
        (Pawn|Input|AddMovementInput (Math|Vector|GetRightVector (Math|Rotator|MakeRotator 0.0 0.0 (.Yaw (Math|Rotator|BreakRotator (Transformation|GetWorldRotation (Variables|Collision|GetCapsuleComponent)))))) (Variables|Default|GetMoveRightAxisValue) false)
        (else
          ;[1 1 1] 기본 이동
          (Pawn|Input|AddMovementInput (Math|Vector|GetRightVector (Math|Rotator|MakeRotator 0.0 0.0 (.Yaw (Math|Rotator|BreakRotator (Pawn|GetControlRotation :!class /Script/Engine.Pawn))))) (Variables|Default|GetMoveRightAxisValue) false))))
    (:MOVE_Swimming
      (goto _label))
    (:MOVE_Flying
      (CallFunction|MoveonWall (Transformation|GetActorRightVector) (Variables|Default|GetMoveRightAxisValue)))))

(event Input|AxisEvents|InputAxisLookUp
  (params (AxisValue :type Float%20%28single-precision%29))
  ;[1 1 1] 캐릭터 마우스 회전
  (Pawn|Input|AddControllerPitchInput AxisValue))

(event Input|AxisEvents|InputAxisTurn
  (params (AxisValue :type Float%20%28single-precision%29))
  ;[1 1 1] 캐릭터 마우스 회전
  (Pawn|Input|AddControllerYawInput AxisValue))

(event EventCallEquipWeaponArea
  (Variables|Default|SetbIsInEquipWeaponArea? true))

(event Input|ActionEvents|InputActionInteraction
  (params (Key :type Key%20Structure))
  (:Pressed
    (if (Variables|Default|GetbIsInEquipWeaponArea?)
      (Rendering|SetVisibility (Variables|Default|GetCharacterWeapon) true false)
      (Variables|Default|SetbIsEquipWeapon? true)
      (Variables|Default|SetbIsEnableCombatCollision? true))))

(fn ConstructionScript)

(fn MoveonWall
  (params (Vector :type Vector) (AxisValue :type Float%20%28single-precision%29))
  (bind _returnvalue (Transformation|GetActorLocation))
  (if (!= AxisValue 0.0)
    (LocalVariables|SetRightCapsuleTraceStart _returnvalue)
    (LocalVariables|SetRightCapsuleTraceEnd (+ _returnvalue (* Vector (* AxisValue 5e+01))))
    (bind (_outhit _returnvalue_2) (Collision|CapsuleTraceByChannel (LocalVariables|GetRightCapsuleTraceStart) (LocalVariables|GetRightCapsuleTraceEnd) 3e+01 96.0 "TraceTypeQuery1" false 0 "None"))
    (if _returnvalue_2
      (LocalVariables|SetMoveTarget (.Location (Collision|BreakHitResult _outhit)))
      (else
        (LocalVariables|SetMoveTarget (LocalVariables|GetRightCapsuleTraceEnd))))
    (bind _linetracechesthit (Utilities|LineTracetoDetactWall (- (LocalVariables|GetMoveTarget) (Transformation|GetActorLocation))))
    (Pawn|Input|AddMovementInput (Math|Vector|MakeVector (.x (Math|Vector|GetUnitDirection(Vector) (Transformation|GetActorLocation) (+ (.Location (Collision|BreakHitResult _linetracechesthit)) (* (.Normal (Collision|BreakHitResult _linetracechesthit)) (Variables|Default|GetClimbingWallDistance))))) (.y (Math|Vector|GetUnitDirection(Vector) (Transformation|GetActorLocation) (+ (.Location (Collision|BreakHitResult _linetracechesthit)) (* (.Normal (Collision|BreakHitResult _linetracechesthit)) (Variables|Default|GetClimbingWallDistance))))) (.z (Math|Vector|GetUnitDirection(Vector) (Transformation|GetActorLocation) (+ (.Location (Collision|BreakHitResult _linetracechesthit)) (* (.Normal (Collision|BreakHitResult _linetracechesthit)) (Variables|Default|GetClimbingWallDistance)))))) 1.0 false)))