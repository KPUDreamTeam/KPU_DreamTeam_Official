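; Player controller for the main character, handling movement, camera look and sprint input.
; Move axes push the player character along forward and right vectors built from control-rotation yaw only, so camera pitch does not affect direction.
; Turn and LookUp axes feed the character's controller yaw and pitch input.
; Sprint casts the player pawn to BP_MainChar and raises its max walk speed while held, restoring walking speed on release.
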(event Input|ActionEvents|InputActionSprint
  (params (Key :type Key%20Structure :default "None"))
  (bind _returnvalue (Game|Player|GetPlayerPawn 0))
  ;[1 1 1] 캐릭터 LeftShift를 통한 뛰기
  (:Pressed
    (bind _asbp_main_char (Utilities|Casting|CastToBP_MainChar _returnvalue))
    (Variables|/Script/Engine.CharacterMovementComponent|SetMaxWalkSpeed (Variables|/Script/Engine.Character|GetCharacterMovement _asbp_main_char) 4.5e+02))
  (:Released
    (bind _asbp_main_char_2 (Utilities|Casting|CastToBP_MainChar _returnvalue))
    (Variables|/Script/Engine.CharacterMovementComponent|SetMaxWalkSpeed (Variables|/Script/Engine.Character|GetCharacterMovement _asbp_main_char_2) 3e+02)))

(event Input|AxisEvents|InputAxisMoveForward
  (params (AxisValue :type Float%20%28single-precision%29))
  ;[1 1 1] 캐릭터 이동 (상,하,좌,우)
  (Pawn|Input|AddMovementInput (Game|GetPlayerCharacter 0) (Math|Vector|GetForwardVector (Math|Rotator|MakeRotator 0.0 0.0 (.Yaw (Math|Rotator|BreakRotator (Pawn|GetControlRotation :!class /Script/Engine.Controller))))) AxisValue false))

(event Input|AxisEvents|InputAxisMoveRight
  (params (AxisValue :type Float%20%28single-precision%29))
  ;[1 1 1] 캐릭터 이동 (상,하,좌,우)
  (Pawn|Input|AddMovementInput (Game|GetPlayerCharacter 0) (Math|Vector|GetRightVector (Math|Rotator|MakeRotator 0.0 0.0 (.Yaw (Math|Rotator|BreakRotator (Pawn|GetControlRotation :!class /Script/Engine.Controller))))) AxisValue false))

(event Input|AxisEvents|InputAxisLookUp
  (params (AxisValue :type Float%20%28single-precision%29))
  ;[1 1 1] 축 이동
  (Pawn|Input|AddControllerPitchInput (Game|GetPlayerCharacter 0) AxisValue))

(event Input|AxisEvents|InputAxisTurn
  (params (AxisValue :type Float%20%28single-precision%29))
  ;[1 1 1] 축 이동
  (Pawn|Input|AddControllerYawInput (Game|GetPlayerCharacter 0) AxisValue))

(fn ConstructionScript)